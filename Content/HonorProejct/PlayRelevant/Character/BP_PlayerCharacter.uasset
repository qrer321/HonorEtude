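; Player character Blueprint that defines a camera transition between combat and non-combat views.
; CombatCameraSwitch checks IsCombatMode and eases the camera boom's offsets, location and arm length, plus follow camera rotation, using frame-delta interpolation.
; Combat mode gives a closer, side-shifted over-the-shoulder view, while the other mode pulls back and raises the camera.
; The event graph's only call to this function is unconnected, and Tick is empty, so the switch never runs from here.
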(event EventBeginPlay)

(event Collision|EventActorBeginOverlap
  (params (OtherActor :type Actor%20Object%20Reference)))

(event EventTick
  (params (DeltaSeconds :type Float%20%28single-precision%29)))

(fn ConstructionScript)

(fn CombatCameraSwitch
  (bind _returnvalue (Utilities|Time|GetWorldDeltaSeconds))
  (bind _returnvalue_2 (Utilities|Time|GetWorldDeltaSeconds))
  (bind _returnvalue_3 (Utilities|Time|GetWorldDeltaSeconds))
  (bind _returnvalue_4 (Utilities|Time|GetWorldDeltaSeconds))
  (bind _returnvalue_5 (Utilities|Time|GetWorldDeltaSeconds))
  (bind _m_cameraboom (Variables|Default|Getm_CameraBoom))
  (bind _m_cameraboom_2 (Variables|Default|Getm_CameraBoom))
  (bind _m_cameraboom_3 (Variables|Default|Getm_CameraBoom))
  (bind _m_cameraboom_4 (Variables|Default|Getm_CameraBoom))
  (bind _m_followcamera (Variables|Default|Getm_FollowCamera))
  (bind _m_followcamera_2 (Variables|Default|Getm_FollowCamera))
  (bind _relativerotation (Variables|/Script/Engine.SceneComponent|GetRelativeRotation _m_followcamera_2))
  (if (Class|HonorProjectCharacter|IsCombatMode)
    (Variables|/Script/Engine.SpringArmComponent|SetTargetOffset _m_cameraboom_2 (Math|Interpolation|VInterpTo (Variables|/Script/Engine.SpringArmComponent|GetTargetOffset (Variables|Default|Getm_CameraBoom)) "0,0.000000,30.000000" _returnvalue_2 5.0))
    (Variables|/Script/Engine.SpringArmComponent|SetSocketOffset _m_cameraboom_3 (Math|Interpolation|VInterpTo (Variables|/Script/Engine.SpringArmComponent|GetSocketOffset _m_cameraboom_2) "0,100.000000, 0" _returnvalue_5 5.0))
    (Transformation|SetRelativeLocation _m_cameraboom_4 (Math|Interpolation|VInterpTo (Variables|/Script/Engine.SceneComponent|GetRelativeLocation _m_cameraboom_3) "0, 0,30.000000" _returnvalue 5.0) false false)
    (Variables|/Script/Engine.SpringArmComponent|SetTargetArmLength _m_cameraboom (Math|Interpolation|FInterpTo (Variables|/Script/Engine.SpringArmComponent|GetTargetArmLength _m_cameraboom_4) 2e+02 _returnvalue_3 5.0))
    (Transformation|SetRelativeRotation _m_followcamera (Math|Interpolation|RInterpTo _relativerotation "0,-10.000000, 0" _returnvalue_4 5.0) false false)
    (else
      (Variables|/Script/Engine.SpringArmComponent|SetTargetOffset _m_cameraboom_2 (Math|Interpolation|VInterpTo (Variables|/Script/Engine.SpringArmComponent|GetTargetOffset (Variables|Default|Getm_CameraBoom)) "0,0.000000,150.000000" _returnvalue_2 5.0))
      (Variables|/Script/Engine.SpringArmComponent|SetSocketOffset _m_cameraboom_3 (Math|Interpolation|VInterpTo (Variables|/Script/Engine.SpringArmComponent|GetSocketOffset _m_cameraboom_2) "0, 0, 0" _returnvalue_5 5.0))
      (Transformation|SetRelativeLocation _m_cameraboom_4 (Math|Interpolation|VInterpTo (Variables|/Script/Engine.SceneComponent|GetRelativeLocation _m_cameraboom_3) "0, 0,80.000000" _returnvalue 5.0) false false)
      (Variables|/Script/Engine.SpringArmComponent|SetTargetArmLength _m_cameraboom (Math|Interpolation|FInterpTo (Variables|/Script/Engine.SpringArmComponent|GetTargetArmLength _m_cameraboom_4) 3e+02 _returnvalue_3 5.0))
      (Transformation|SetRelativeRotation _m_followcamera (Math|Interpolation|RInterpTo _relativerotation "-30.000000,0.000000, 0" _returnvalue_4 5.0) false false))))