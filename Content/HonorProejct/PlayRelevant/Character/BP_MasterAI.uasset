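; Base AI character, by its name the parent for AI pawns, that tracks the player as a target and carries a sword.
; PawnSensing stores a seen BP_PlayerCharacter as TargetCharacter, and a Tick check clears it once its distance exceeds the sight radius.
; Tick also spins the visible target decal.
; Helpers snap the sword to a named mesh socket and convert the strafing enum to an actor-relative vector; damage only prints a debug string.
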(event EventBeginPlay)

(event Collision|EventActorBeginOverlap
  (params (OtherActor :type Actor%20Object%20Reference)))

(event EventTick
  (params (DeltaSeconds :type Float%20%28single-precision%29))
  (bind _m_targetdecal (Variables|Default|Getm_TargetDecal))
  (CallFunction|IsTargetDisappear?)
  (if (Rendering|IsVisible _m_targetdecal)
    (Transformation|AddWorldRotation _m_targetdecal "0.000000,1.000000, 0" false false)))

(event Game|Damage|EventAnyDamage
  (params (Damage :type Float%20%28single-precision%29) (DamageType :type Damage%20Type%20Object%20Reference) (InstigatedBy :type Controller%20Object%20Reference) (DamageCauser :type Actor%20Object%20Reference))
  (Development|PrintString "Any Damage"))

(event EventSetWeaponSocketLocation
  (params (SocketName :type Name :default "None"))
  (Transformation|AttachComponentToComponent (Variables|Default|GetSwordMesh) (Variables|Character|GetMesh) SocketName "SnapToTarget" "SnapToTarget" "SnapToTarget" true))

(event OnSeePawn(PawnSensing)
  (params (Pawn :type Pawn%20Object%20Reference))
  (bind _asbp_player_character (Utilities|Casting|CastToBP_PlayerCharacter Pawn))
  (Variables|Default|SetTargetCharacter _asbp_player_character))

(event Custom|IsTargetDisappear?
  (Utilities|IsValid (Variables|Default|GetTargetCharacter)
    (:Is%20Valid
      (if (< (Variables|/Script/AIModule.PawnSensingComponent|GetSightRadius (Variables|Default|GetPawnSensing)) (Transformation|GetDistanceTo (Variables|Default|GetTargetCharacter)))
        (Variables|Default|SetTargetCharacter 0)))))

(fn ConstructionScript)

(fn SetStrafingDirection
  (bind _self self)
  (bind _self_2 self)
  (bind _returnvalue (Transformation|GetActorForwardVector _self_2))
  (bind _returnvalue_2 (Transformation|GetActorRightVector _self))
  (switch Utilities|FlowControl|Switch|SwitchonE_StrafingDirection (Variables|Default|GetEStrafingDirection)
    (:NewEnumerator3
      (Variables|Default|SetStrafingDirectionVector _returnvalue))
    (:NewEnumerator0
      (Variables|Default|SetStrafingDirectionVector (* _returnvalue -1.0)))
    (:NewEnumerator1
      (Variables|Default|SetStrafingDirectionVector _returnvalue_2))
    (:NewEnumerator2
      (Variables|Default|SetStrafingDirectionVector (* _returnvalue_2 -1.0))))
  (return (Variables|Default|GetStrafingDirectionVector)))