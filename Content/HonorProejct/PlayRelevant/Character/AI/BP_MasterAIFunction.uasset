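; Shared AI helper functions for master AI pawns that target the player character.
; A cast helper resolves the pawn to BP_MasterAI and reads the player from the controller's blackboard target key, printing a message on failure.
; The distance function uses that helper to write the mesh-to-mesh distance back to the blackboard.
; A separate function instantly turns the AI actor to face the player with a look-at rotation.
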(fn CastAIandPlayerCharacter
  (params (Master%20AI%20Pawn :type Object%20Object%20Reference) (Master%20AI%20Controller :type AI%20Controller%20Object%20Reference))
  (bind _asbp_master_ai (Utilities|Casting|CastToBP_MasterAI Master%20AI%20Pawn)
    (:then
      (LocalVariables|SetAI%20Character _asbp_master_ai)
      (bind _asbp_player_character (Utilities|Casting|CastToBP_PlayerCharacter (AI|Components|Blackboard|GetValueasObject (AI|GetBlackboard Master%20AI%20Controller) (LocalVariables|GetTargetKey)))
        (:then
          (bind _output_get (LocalVariables|SetTarget%20Character _asbp_player_character))
          (return (LocalVariables|GetAI%20Character) _output_get))
        (:CastFailed
          (Development|PrintString 0 "PlayerCharacter Failed"))))
    (:CastFailed
      (Development|PrintString 0 "MasterAI Failed"))))

(fn TargetDistanceCalc
  (params (AI%20Controller :type AI%20Controller%20Object%20Reference) (Controlled%20Pawn :type Pawn%20Object%20Reference))
  (bind (_master_ai_character _player_character) (CallFunction|CastAIandPlayerCharacter Controlled%20Pawn AI%20Controller))
  (LocalVariables|SetMaster%20AI%20Character _master_ai_character)
  (LocalVariables|SetPlayer%20Character _player_character)
  (AI|Components|Blackboard|SetValueasFloat (AI|GetBlackboard (AI|GetAIController (LocalVariables|GetMaster%20AI%20Character))) (LocalVariables|GetAI%20To%20Player%20Distance%20Diff) (Math|Vector|Distance(Vector) (Transformation|GetWorldLocation (Variables|/Script/Engine.Character|GetMesh (LocalVariables|GetMaster%20AI%20Character))) (Transformation|GetWorldLocation (Variables|/Script/Engine.Character|GetMesh (LocalVariables|GetPlayer%20Character))))))

(fn RotatetoTarget
  (params (Master%20AI%20Character :type BP%20Master%20AI%20Object%20Reference) (Player%20Character :type Player%20Character%20Object%20Reference))
  (Utilities|IsValid Master%20AI%20Character
    (:Is%20Valid
      (Utilities|IsValid Player%20Character
        (:Is%20Valid
          (Transformation|SetActorRotation Master%20AI%20Character (Math|Rotator|FindLookatRotation (Transformation|GetActorLocation Master%20AI%20Character) (Transformation|GetActorLocation Player%20Character))))))))